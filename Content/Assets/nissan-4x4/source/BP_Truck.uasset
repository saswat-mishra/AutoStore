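; Showroom truck actor that opens a WBP_Configurator widget while its capsule is overlapped.
; Widget events drive body colour and headlight material swaps, wheel movement, marker visibility and a switch to the Cam view, which hides the character.
; Tick handles optional turntable yaw, back-and-forth sweeping of the Sphere components and pulsing marker scale.
; Markers highlight on hover and open lights, interior or wheels details on click, while character input events rotate Cam.
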(event `self.ReceiveTick`
  (params (DeltaSeconds :type "Float (single-precision)"))
  (bind (_returnvalue_roll _returnvalue_pitch _returnvalue_yaw) (`KismetMathLibrary.BreakRotator` (`self.K2_GetActorRotation`)))
  (bind _returnvalue (* DeltaSeconds 10.0))
  (bind _returnvalue_2 (* (0.08 0.08 0.08) DeltaSeconds))
  (bind _marker1 (`self.marker1`))
  (bind _sphere (`self.Sphere`))
  (bind _relativescale3d (`SceneComponent.RelativeScale3D` _marker1))
  (bind (_relativerotation_roll _relativerotation_pitch _relativerotation_yaw) (`KismetMathLibrary.BreakRotator` (`SceneComponent.RelativeRotation` _sphere)))
  (bind _x (.x _relativescale3d))
  (`|ExecutionSequence`
    (:`then_0`
      (if (`self.rotate?`)
        (`self.K2_SetActorRotation` (`KismetMathLibrary.MakeRotator` _returnvalue_roll _returnvalue_pitch (+ _returnvalue_yaw (* DeltaSeconds 10.0))))))
    (:`then_1`
      (if (`self.moveWheel`)
        (if (`self.revWheel`)
          (`SceneComponent.K2_SetRelativeRotation` _sphere (`KismetMathLibrary.MakeRotator` _relativerotation_roll _relativerotation_pitch (+ _relativerotation_yaw _returnvalue)) false false)
          (`SceneComponent.K2_SetRelativeRotation` (`self.Sphere1`) (`KismetMathLibrary.MakeRotator` _relativerotation_roll _relativerotation_pitch (+ _relativerotation_yaw _returnvalue)) false false)
          (if (>= _relativerotation_yaw 30.0)
            (set `self.revWheel` false))
          (else
            (`SceneComponent.K2_SetRelativeRotation` _sphere (`KismetMathLibrary.MakeRotator` _relativerotation_roll _relativerotation_pitch (- _relativerotation_yaw _returnvalue)) false false)
            (`SceneComponent.K2_SetRelativeRotation` (`self.Sphere1`) (`KismetMathLibrary.MakeRotator` _relativerotation_roll _relativerotation_pitch (- _relativerotation_yaw _returnvalue)) false false)
            (if (<= _relativerotation_yaw -30.0)
              (set `self.revWheel` true))))))
    (:`then_2`
      (if (`self.blinkMarker`)
        (if (`self.enlarge`)
          (`SceneComponent.SetRelativeScale3D` _marker1 (+ _relativescale3d _returnvalue_2))
          (`SceneComponent.SetRelativeScale3D` (`self.marker5`) (+ _relativescale3d _returnvalue_2))
          (`SceneComponent.SetRelativeScale3D` (`self.marker4`) (+ _relativescale3d _returnvalue_2))
          (`SceneComponent.SetRelativeScale3D` (`self.marker3`) (+ _relativescale3d _returnvalue_2))
          (`SceneComponent.SetRelativeScale3D` (`self.marker2`) (+ _relativescale3d _returnvalue_2))
          (`SceneComponent.SetRelativeScale3D` (`self.marker`) (+ _relativescale3d _returnvalue_2))
          (if (> _x 0.2)
            (set `self.enlarge` false))
          (else
            (`SceneComponent.SetRelativeScale3D` _marker1 (- _relativescale3d _returnvalue_2))
            (`SceneComponent.SetRelativeScale3D` (`self.marker5`) (- _relativescale3d _returnvalue_2))
            (`SceneComponent.SetRelativeScale3D` (`self.marker4`) (- _relativescale3d _returnvalue_2))
            (`SceneComponent.SetRelativeScale3D` (`self.marker3`) (- _relativescale3d _returnvalue_2))
            (`SceneComponent.SetRelativeScale3D` (`self.marker2`) (- _relativescale3d _returnvalue_2))
            (`SceneComponent.SetRelativeScale3D` (`self.marker`) (- _relativescale3d _returnvalue_2))
            (if (< _x 0.1)
              (set `self.enlarge` true))))))))

(event `self.ReceiveBeginPlay`
  (bind _asbp_third_person_character (cast `/Game/ThirdPerson/Blueprints/BP_ThirdPersonCharacter` (`GameplayStatics.GetPlayerCharacter` 0)))
  (bind _output_get (set `self.As BP Third Person Character` _asbp_third_person_character))
  (add `/Game/ThirdPerson/Blueprints/BP_ThirdPersonCharacter.add Camera Rotation` _output_get (delegate `set Camera Yaw`)))

(event `set Camera Yaw`
  (params (Val :type "Rotator Structure"))
  (`SceneComponent.K2_AddRelativeRotation` (`CameraActor.CameraComponent` (`self.cam`)) (* Val 5.0) false false))

(event `self.Capsule.OnComponentBeginOverlap`
  (params (OverlappedComponent :type "PrimitiveComponent Object Reference") (OtherActor :type "Actor Object Reference") (OtherComp :type "PrimitiveComponent Object Reference") (OtherBodyIndex :type Integer) (bFromSweep :type Boolean) (SweepResult :type "HitResult Structure (by ref)"))
  (bind _returnvalue (`|CreateWidget` "/Game/Widgets/WBP_Configurator.WBP_Configurator_C" (`GameplayStatics.GetPlayerController` 0)))
  (bind _output_get (set `self.Config` _returnvalue))
  (`UserWidget.AddToViewport` _output_get 0)
  (`Widget.SetIsEnabled` (`/Game/Widgets/WBP_Configurator.Button_2` _output_get) (not (`self.rotate?`)))
  (set `/Game/Widgets/WBP_Configurator.vehicleType` "truck" _output_get)
  (add `/Game/Widgets/WBP_Configurator.moveWheels` _output_get (delegate `moveWheels`))
  (add `/Game/Widgets/WBP_Configurator.switchOnHeadlight` _output_get (delegate `LightsOn`))
  (add `/Game/Widgets/WBP_Configurator.changeColour` _output_get (delegate `changeColour`))
  (add `/Game/Widgets/WBP_Configurator.changeView` _output_get (delegate `setView`))
  (add `/Game/Widgets/WBP_Configurator.showMarker` _output_get (delegate `showMarkers`)))

(event `setView`
  (params (FPV :type Boolean))
  (bind _as_bp_third_person_character (`self.As BP Third Person Character`))
  (if FPV
    (`PlayerController.SetViewTargetWithBlend` (`GameplayStatics.GetPlayerController` 0) (`self.cam`) 0.0 "VTBlend_Linear" 0.0 false)
    (set `/Game/ThirdPerson/Blueprints/BP_ThirdPersonCharacter.shouldCharMove` false _as_bp_third_person_character)
    (`self.SetActorHiddenInGame` _as_bp_third_person_character true)
    (else
      (`PlayerController.SetViewTargetWithBlend` (`GameplayStatics.GetPlayerController` 0) (`GameplayStatics.GetPlayerCharacter` 0) 0.0 "VTBlend_Linear" 0.0 false)
      (set `/Game/ThirdPerson/Blueprints/BP_ThirdPersonCharacter.shouldCharMove` true _as_bp_third_person_character)
      (`self.SetActorHiddenInGame` _as_bp_third_person_character false))))

(event `moveWheels`
  (params (move :type Boolean))
  (set `self.moveWheel` move))

(event `showMarkers`
  (params (show :type Boolean))
  (bind _marker3 (`self.marker3`))
  (set `self.blinkMarker` show)
  (if show
    (`SceneComponent.SetHiddenInGame` _marker3 false false)
    (`SceneComponent.SetHiddenInGame` (`self.marker4`) false false)
    (`SceneComponent.SetHiddenInGame` (`self.marker5`) false false)
    (`SceneComponent.SetHiddenInGame` (`self.marker1`) false false)
    (`SceneComponent.SetHiddenInGame` (`self.marker`) false false)
    (`SceneComponent.SetHiddenInGame` (`self.marker2`) false false)
    (else
      (`SceneComponent.SetHiddenInGame` _marker3 true false)
      (`SceneComponent.SetHiddenInGame` (`self.marker4`) true false)
      (`SceneComponent.SetHiddenInGame` (`self.marker5`) true false)
      (`SceneComponent.SetHiddenInGame` (`self.marker1`) true false)
      (`SceneComponent.SetHiddenInGame` (`self.marker`) true false)
      (`SceneComponent.SetHiddenInGame` (`self.marker2`) true false))))

(event `LightsOn`
  (params (on :type Boolean))
  (bind _nissan4x4_pickup_005 (`self.Nissan4x4_pickup_005`))
  (if on
    (`PrimitiveComponent.SetMaterial` _nissan4x4_pickup_005 0 "/Game/Assets/LED_Ceiling_Light/LED_Ceiling_Light/light.light")
    (else
      (`PrimitiveComponent.SetMaterial` _nissan4x4_pickup_005 0 "/Engine/BasicShapes/BasicShapeMaterial.BasicShapeMaterial"))))

(event `self.Capsule.OnComponentEndOverlap`
  (params (OverlappedComponent :type "PrimitiveComponent Object Reference") (OtherActor :type "Actor Object Reference") (OtherComp :type "PrimitiveComponent Object Reference") (OtherBodyIndex :type Integer))
  (`Widget.RemoveFromParent` (`self.Config`)))

(event `changeColour`
  (params (colour :type String))
  (bind _nissan4x4_body (`self.Nissan4x4_body`))
  (if (`KismetStringLibrary.EqualEqual_StrStr` colour "yellow")
    (`PrimitiveComponent.SetMaterial` _nissan4x4_body 0 "/Game/Materials/YellowTruck.YellowTruck")
    (elif (`KismetStringLibrary.EqualEqual_StrStr` colour "blue")
      (`PrimitiveComponent.SetMaterial` _nissan4x4_body 0 "/Game/Materials/BlueTruck.BlueTruck")
      (elif (`KismetStringLibrary.EqualEqual_StrStr` colour "purple")
        (`PrimitiveComponent.SetMaterial` _nissan4x4_body 0 "/Game/Materials/VioletTruck.VioletTruck")
        (elif (`KismetStringLibrary.EqualEqual_StrStr` colour "black")
          (`PrimitiveComponent.SetMaterial` _nissan4x4_body 0 "/Game/Materials/BlackTruck.BlackTruck")
          (elif (`KismetStringLibrary.EqualEqual_StrStr` colour "white")
            (`PrimitiveComponent.SetMaterial` _nissan4x4_body 0 "/Game/Materials/WhiteTruck.WhiteTruck")
            (elif (`KismetStringLibrary.EqualEqual_StrStr` colour "red")
              (`PrimitiveComponent.SetMaterial` _nissan4x4_body 0 "/Game/Assets/nissan-4x4/source/carpaint.carpaint"))))))))

(event `self.marker1.OnClicked`
  (params (TouchedComponent :type "PrimitiveComponent Object Reference") (ButtonPressed :type "Key Structure"))
  (`/Game/Widgets/WBP_Configurator.open Parts Details` (`self.Config`) "lights" :!label _label))

(event `self.marker3.OnBeginCursorOver`
  (params (TouchedComponent :type "PrimitiveComponent Object Reference"))
  (`PrimitiveComponent.SetMaterial` TouchedComponent 0 "/Game/Materials/SelectedMarkerMat.SelectedMarkerMat"))

(event `self.marker3.OnEndCursorOver`
  (params (TouchedComponent :type "PrimitiveComponent Object Reference"))
  (`PrimitiveComponent.SetMaterial` TouchedComponent 0 "/Engine/VREditor/UI/DiscMaterial.DiscMaterial"))

(event `self.marker.OnClicked`
  (params (TouchedComponent :type "PrimitiveComponent Object Reference") (ButtonPressed :type "Key Structure"))
  (goto _label))

(event `self.marker.OnBeginCursorOver`
  (params (TouchedComponent :type "PrimitiveComponent Object Reference"))
  (`PrimitiveComponent.SetMaterial` TouchedComponent 0 "/Game/Materials/SelectedMarkerMat.SelectedMarkerMat"))

(event `self.marker2.OnClicked`
  (params (TouchedComponent :type "PrimitiveComponent Object Reference") (ButtonPressed :type "Key Structure"))
  (`/Game/Widgets/WBP_Configurator.open Parts Details` (`self.Config`) "interior" :!label _label_2))

(event `self.marker.OnEndCursorOver`
  (params (TouchedComponent :type "PrimitiveComponent Object Reference"))
  (`PrimitiveComponent.SetMaterial` TouchedComponent 0 "/Engine/VREditor/UI/DiscMaterial.DiscMaterial"))

(event `self.marker3.OnClicked`
  (params (TouchedComponent :type "PrimitiveComponent Object Reference") (ButtonPressed :type "Key Structure"))
  (goto _label_2))

(event `self.marker1.OnBeginCursorOver`
  (params (TouchedComponent :type "PrimitiveComponent Object Reference"))
  (`PrimitiveComponent.SetMaterial` TouchedComponent 0 "/Game/Materials/SelectedMarkerMat.SelectedMarkerMat"))

(event `self.marker5.OnClicked`
  (params (TouchedComponent :type "PrimitiveComponent Object Reference") (ButtonPressed :type "Key Structure"))
  (`/Game/Widgets/WBP_Configurator.open Parts Details` (`self.Config`) "wheels" :!label _label_3))

(event `self.marker1.OnEndCursorOver`
  (params (TouchedComponent :type "PrimitiveComponent Object Reference"))
  (`PrimitiveComponent.SetMaterial` TouchedComponent 0 "/Engine/VREditor/UI/DiscMaterial.DiscMaterial"))

(event `self.marker4.OnClicked`
  (params (TouchedComponent :type "PrimitiveComponent Object Reference") (ButtonPressed :type "Key Structure"))
  (goto _label_3))

(event `self.marker2.OnBeginCursorOver`
  (params (TouchedComponent :type "PrimitiveComponent Object Reference"))
  (`PrimitiveComponent.SetMaterial` TouchedComponent 0 "/Game/Materials/SelectedMarkerMat.SelectedMarkerMat"))

(event `self.marker2.OnEndCursorOver`
  (params (TouchedComponent :type "PrimitiveComponent Object Reference"))
  (`PrimitiveComponent.SetMaterial` TouchedComponent 0 "/Engine/VREditor/UI/DiscMaterial.DiscMaterial"))

(event `self.marker4.OnBeginCursorOver`
  (params (TouchedComponent :type "PrimitiveComponent Object Reference"))
  (`PrimitiveComponent.SetMaterial` TouchedComponent 0 "/Game/Materials/SelectedMarkerMat.SelectedMarkerMat"))

(event `self.marker4.OnEndCursorOver`
  (params (TouchedComponent :type "PrimitiveComponent Object Reference"))
  (`PrimitiveComponent.SetMaterial` TouchedComponent 0 "/Engine/VREditor/UI/DiscMaterial.DiscMaterial"))

(event `self.marker5.OnBeginCursorOver`
  (params (TouchedComponent :type "PrimitiveComponent Object Reference"))
  (`PrimitiveComponent.SetMaterial` TouchedComponent 0 "/Game/Materials/SelectedMarkerMat.SelectedMarkerMat"))

(event `self.marker5.OnEndCursorOver`
  (params (TouchedComponent :type "PrimitiveComponent Object Reference"))
  (`PrimitiveComponent.SetMaterial` TouchedComponent 0 "/Engine/VREditor/UI/DiscMaterial.DiscMaterial"))

(fn `UserConstructionScript`)